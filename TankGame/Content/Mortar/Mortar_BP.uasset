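; Mortar Blueprint for an aiming, projectile-firing mortar emplacement with a health bar widget.
; On BeginPlay it initializes the TankAiming component with its barrel, turret and Projectile_BP class, then hands itself to the HealthBar widget from its Widget component.
; The construction script assigns the dome and barrel meshes to the Turret and TankBarrel components, reusing the tank aiming setup for the mortar.
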(event EventBeginPlay
  (Class|TankAimingComponent|Initialize (Variables|Default|GetTankAiming) (Variables|Default|GetTankBarrel) (Variables|Default|GetTurret) "/Game/Projectile/Projectile_BP.Projectile_BP_C")
  (bind _ashealth_bar (Utilities|Casting|CastToHealthBar (UserInterface|GetUserWidgetObject (Variables|Default|GetWidget))))
  (Variables|/Game/UI/HealthBar.HealthBar_C|SetMortar _ashealth_bar self))

(fn ConstructionScript
  (Components|StaticMesh|SetStaticMesh (Variables|Default|GetTurret) "/Game/Mortar/mortar_dome.mortar_dome")
  (Components|StaticMesh|SetStaticMesh (Variables|Default|GetTankBarrel) "/Game/Mortar/mortar_barrel.mortar_barrel"))